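; Stats component for the player character and training dummy, tracking health, plus stamina, XP and level for the player.
; On BeginPlay it casts its owner to pick the player HUD or dummy health bar, then initializes it.
; Each change function updates the widgets directly; decrease functions return whether the stat is depleted.
; XP overflow loops through level-ups, each raising the XP threshold and playing sounds.
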(event EventBeginPlay
  (Utilities|FlowControl|DelayUntilNextTick)
  (bind _asbp_third_person_character (Utilities|Casting|CastToBP_ThirdPersonCharacter (Components|GetOwner))
    (:then
      (Variables|Default|SetPlayer%20Character%20BP _asbp_third_person_character)
      ;[0.05098 0.05098 0.05098] Set Health and Stamina UI
      (Variables|Default|SetIsPlayer true)
      (Progress|SetPercent (Variables|/Game/UI/WB_HUD.WB_HUD_C|GetStaminaBar (Variables|/Game/ThirdPerson/Blueprints/BP_ThirdPersonCharacter.BP_ThirdPersonCharacter_C|GetHUD%20Widget (Variables|Default|GetPlayer%20Character%20BP))) (/ (Variables|Stamina|GetCurrent%20Stamina) (Variables|Stamina|GetMax%20Stamina))))
    (:CastFailed
      (bind _asbp_dummy (Utilities|Casting|CastToBP_Dummy (Components|GetOwner)))
      (Variables|Default|SetDummy%20BP _asbp_dummy)
      (Variables|Default|SetIsPlayer false)))
  (Progress|SetPercent (select (Variables|Default|GetIsPlayer) (Variables|/Game/UI/WB_HUD.WB_HUD_C|GetHealthBar (Variables|/Game/ThirdPerson/Blueprints/BP_ThirdPersonCharacter.BP_ThirdPersonCharacter_C|GetHUD%20Widget (Variables|Default|GetPlayer%20Character%20BP))) (Variables|/Game/UI/WB_DummyHealthBar.WB_DummyHealthBar_C|GetHealthBar (Variables|/Game/Blueprints/BP_Dummy.BP_Dummy_C|GetHealth%20Bar%20UI (Variables|Default|GetDummy%20BP)))) (/ (Variables|Health|GetCurrent%20Health) (Variables|Health|GetMax%20Health)))
  (Rendering|Components|TextRender|SetText (select (Variables|Default|GetIsPlayer) (Variables|/Game/UI/WB_HUD.WB_HUD_C|GetHealthtext (Variables|/Game/ThirdPerson/Blueprints/BP_ThirdPersonCharacter.BP_ThirdPersonCharacter_C|GetHUD%20Widget (Variables|Default|GetPlayer%20Character%20BP))) (Variables|/Game/UI/WB_DummyHealthBar.WB_DummyHealthBar_C|GetHealthText (Variables|/Game/Blueprints/BP_Dummy.BP_Dummy_C|GetHealth%20Bar%20UI (Variables|Default|GetDummy%20BP)))) (Utilities|Text|ToText(Float) (Variables|Health|GetCurrent%20Health) "HalfToEven"))
  ;[0.05098 0.05098 0.05098] Set XP UI
  (if (Variables|Default|GetIsPlayer)
    (Progress|SetPercent (Variables|/Game/UI/WB_HUD.WB_HUD_C|GetXPbar (Variables|/Game/ThirdPerson/Blueprints/BP_ThirdPersonCharacter.BP_ThirdPersonCharacter_C|GetHUD%20Widget (Variables|Default|GetPlayer%20Character%20BP))) (/ (Variables|XP|GetXP) (Variables|XP|GetMax%20XP)))
    (Rendering|Components|TextRender|SetText (Variables|/Game/UI/WB_HUD.WB_HUD_C|GetXPText (Variables|/Game/ThirdPerson/Blueprints/BP_ThirdPersonCharacter.BP_ThirdPersonCharacter_C|GetHUD%20Widget (Variables|Default|GetPlayer%20Character%20BP))) (Utilities|Text|FormatText "{XP} / {MAX}" (Variables|XP|GetXP) (Variables|XP|GetMax%20XP)))
    ;[0.05098 0.05098 0.05098] Set Level UI
    (Rendering|Components|TextRender|SetText (Variables|/Game/UI/WB_HUD.WB_HUD_C|GetLevelText (Variables|/Game/ThirdPerson/Blueprints/BP_ThirdPersonCharacter.BP_ThirdPersonCharacter_C|GetHUD%20Widget (Variables|Default|GetPlayer%20Character%20BP))) (Utilities|Text|ToText(Integer) (Variables|XP|GetLevel)))))

(event EventTick
  (params (DeltaSeconds :type Float%20%28single-precision%29)))

(fn DecreaseHealth
  (params (Damage :type Float%20%28double-precision%29))
  (bind _player_character_bp (Variables|Default|GetPlayer%20Character%20BP))
  (bind _dummy_bp (Variables|Default|GetDummy%20BP))
  (bind _isplayer (Variables|Default|GetIsPlayer))
  (bind _hud_widget (Variables|/Game/ThirdPerson/Blueprints/BP_ThirdPersonCharacter.BP_ThirdPersonCharacter_C|GetHUD%20Widget _player_character_bp))
  (bind _health_bar_ui (Variables|/Game/Blueprints/BP_Dummy.BP_Dummy_C|GetHealth%20Bar%20UI _dummy_bp))
  (bind _healthtext (Variables|/Game/UI/WB_DummyHealthBar.WB_DummyHealthBar_C|GetHealthText _health_bar_ui))
  (bind _healthtext_2 (Variables|/Game/UI/WB_HUD.WB_HUD_C|GetHealthtext _hud_widget))
  (bind _returnvalue (select _isplayer _healthtext_2 _healthtext))
  (if (<= (Variables|Health|GetCurrent%20Health) 0.0)
    (return true)
    (else
      (bind _output_get (Variables|Health|SetCurrent%20Health (- (Variables|Health|GetCurrent%20Health) Damage)))
      (Progress|SetPercent (select _isplayer (Variables|/Game/UI/WB_HUD.WB_HUD_C|GetHealthBar _hud_widget) (Variables|/Game/UI/WB_DummyHealthBar.WB_DummyHealthBar_C|GetHealthBar _health_bar_ui)) (/ _output_get (Variables|Health|GetMax%20Health)))
      (if (<= (Variables|Health|GetCurrent%20Health) 0.0)
        (Rendering|Components|TextRender|SetText _returnvalue "0")
        (if (Variables|Default|GetIsPlayer)
          _
          (else
            (Variables|/Script/UMG.Widget|SetVisibility (Variables|/Game/Blueprints/BP_Dummy.BP_Dummy_C|GetHealth%20Bar%20UI (Variables|Default|GetDummy%20BP)) "Hidden")))
        (return true)
        (else
          (Rendering|Components|TextRender|SetText _returnvalue (Utilities|Text|ToText(Float) (Variables|Health|GetCurrent%20Health) "HalfToEven"))
          (return false))))))

(fn IncreaseMaxHealth
  (params (Increment :type Float%20%28double-precision%29))
  (bind _output_get (Variables|Health|SetMax%20Health (+ Increment (Variables|Health|GetMax%20Health))))
  (Progress|SetPercent (Variables|/Game/UI/WB_HUD.WB_HUD_C|GetHealthBar (Variables|/Game/ThirdPerson/Blueprints/BP_ThirdPersonCharacter.BP_ThirdPersonCharacter_C|GetHUD%20Widget (Variables|Default|GetPlayer%20Character%20BP))) (/ (Variables|Health|GetCurrent%20Health) _output_get)))

(fn DecreaseStamina
  (params (Stamina%20decrease :type Float%20%28double-precision%29))
  (if (<= (Variables|Stamina|GetCurrent%20Stamina) 0.0)
    (return true)
    (else
      (bind _output_get (Variables|Stamina|SetCurrent%20Stamina (- (Variables|Stamina|GetCurrent%20Stamina) Stamina%20decrease)))
      (Progress|SetPercent (Variables|/Game/UI/WB_HUD.WB_HUD_C|GetStaminaBar (Variables|/Game/ThirdPerson/Blueprints/BP_ThirdPersonCharacter.BP_ThirdPersonCharacter_C|GetHUD%20Widget (Variables|Default|GetPlayer%20Character%20BP))) (/ _output_get (Variables|Stamina|GetMax%20Stamina)))
      (if (<= (Variables|Stamina|GetCurrent%20Stamina) 0.0)
        (return true)
        (else
          (return false))))))

(fn IncreaseMaxStamina
  (params (Increase :type Float%20%28double-precision%29))
  (Variables|Stamina|SetMax%20Stamina (+ Increase (Variables|Health|GetMax%20Health)))
  (Progress|SetPercent (Variables|/Game/UI/WB_HUD.WB_HUD_C|GetStaminaBar (Variables|/Game/ThirdPerson/Blueprints/BP_ThirdPersonCharacter.BP_ThirdPersonCharacter_C|GetHUD%20Widget (Variables|Default|GetPlayer%20Character%20BP))) (/ (Variables|Stamina|GetCurrent%20Stamina) (Variables|Stamina|GetMax%20Stamina))))

(fn IncreaseHealth
  (params (Heal%20amount :type Float%20%28double-precision%29))
  (bind _max_health (Variables|Health|GetMax%20Health))
  (bind _player_character_bp (Variables|Default|GetPlayer%20Character%20BP))
  (bind _hud_widget (Variables|/Game/ThirdPerson/Blueprints/BP_ThirdPersonCharacter.BP_ThirdPersonCharacter_C|GetHUD%20Widget _player_character_bp))
  (bind _output_get (Variables|Health|SetCurrent%20Health (+ Heal%20amount (Variables|Health|GetCurrent%20Health))))
  (if (> _output_get _max_health)
    (Variables|Health|SetCurrent%20Health (Variables|Health|GetMax%20Health)))
  (Progress|SetPercent (Variables|/Game/UI/WB_HUD.WB_HUD_C|GetHealthBar _hud_widget) (/ (Variables|Health|GetCurrent%20Health) _max_health))
  (Rendering|Components|TextRender|SetText (Variables|/Game/UI/WB_HUD.WB_HUD_C|GetHealthtext _hud_widget) (Utilities|Text|ToText(Float) (Variables|Health|GetCurrent%20Health) "HalfToEven")))

(fn IncreaseStamina
  (params (added%20stamina :type Float%20%28double-precision%29))
  (bind _max_stamina (Variables|Stamina|GetMax%20Stamina))
  (bind _player_character_bp (Variables|Default|GetPlayer%20Character%20BP))
  (if (Utilities|IsValid _player_character_bp)
    (bind _output_get (Variables|Stamina|SetCurrent%20Stamina (+ added%20stamina (Variables|Stamina|GetCurrent%20Stamina))))
    (if (> _output_get _max_stamina)
      (Variables|Stamina|SetCurrent%20Stamina _max_stamina))
    (Progress|SetPercent (Variables|/Game/UI/WB_HUD.WB_HUD_C|GetStaminaBar (Variables|/Game/ThirdPerson/Blueprints/BP_ThirdPersonCharacter.BP_ThirdPersonCharacter_C|GetHUD%20Widget _player_character_bp)) (/ (Variables|Stamina|GetCurrent%20Stamina) (Variables|Stamina|GetMax%20Stamina)))))

(fn IncreaseXP
  (params (Add%20XP :type Float%20%28double-precision%29))
  (bind _player_character_bp (Variables|Default|GetPlayer%20Character%20BP))
  (bind _hud_widget (Variables|/Game/ThirdPerson/Blueprints/BP_ThirdPersonCharacter.BP_ThirdPersonCharacter_C|GetHUD%20Widget _player_character_bp))
  (Variables|XP|SetXP (+ Add%20XP (Variables|XP|GetXP)))
  (if (>= (Variables|XP|GetXP) (Variables|XP|GetMax%20XP)) :!label _label
    (Variables|XP|SetXP (- (Variables|XP|GetXP) (Variables|XP|GetMax%20XP)))
    (XP|IncreaseLevel 1)
    (goto _label)
    (else
      (Progress|SetPercent (Variables|/Game/UI/WB_HUD.WB_HUD_C|GetXPbar _hud_widget) (/ (Variables|XP|GetXP) (Variables|XP|GetMax%20XP)))
      (Rendering|Components|TextRender|SetText (Variables|/Game/UI/WB_HUD.WB_HUD_C|GetXPText _hud_widget) (Utilities|Text|FormatText "{XP} / {MAX}" (Variables|XP|GetXP) (Variables|XP|GetMax%20XP))))))

(fn IncreaseLevel
  (params (Add%20Level :type Integer))
  (Variables|XP|SetLevel (+ Add%20Level (Variables|XP|GetLevel)))
  (Variables|XP|SetMax%20XP (+ (Variables|XP|GetMax%20XP) 1.5e+02))
  (Rendering|Components|TextRender|SetText (Variables|/Game/UI/WB_HUD.WB_HUD_C|GetLevelText (Variables|/Game/ThirdPerson/Blueprints/BP_ThirdPersonCharacter.BP_ThirdPersonCharacter_C|GetHUD%20Widget (Variables|Default|GetPlayer%20Character%20BP))) (Utilities|Text|ToText(Integer) (Variables|XP|GetLevel)))
  (Audio|PlaySound2D "/Game/Audio/UI/LevelUp.LevelUp" 1.0 1.0 0.0 0 0)
  (Audio|PlaySound2D "/Game/Audio/UI/475889__epicsoundeffects__ese-whoosh-epic-level-up.475889__epicsoundeffects__ese-whoosh-epic-level-up" 1.0 1.0 0.0 0 0))